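; Player controller that flies a DefaultPawn with PlayStation gamepad input through Enhanced Input.
; On BeginPlay it adds the gamepad mappable config, scans and prints registered devices, and sets game-only input.
; A device name containing product code 05C4 sets a first-generation DualShock 4 flag, which this graph never reads.
; Look and Roll actions drive controller rotation, while Move drives the pawn's right, forward and world-up movement.
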(event Input|EnhancedActionEvents|EnhancedInputActionIA_PSGamepad_Roll
  (params (ActionValue :type Float%20%28double-precision%29) (ElapsedSeconds :type Float%20%28double-precision%29) (TriggeredSeconds :type Float%20%28double-precision%29) (InputAction :type Input%20Action%20Object%20Reference :default "/Game/PlaystationGamepad/IA_PSGamepad_Roll.IA_PSGamepad_Roll"))
  (:Triggered
    (Class|PlayerController|AddRollInput ActionValue :!label _label))
  (:Ongoing
    (goto _label)))

(event Input|EnhancedActionEvents|EnhancedInputActionIA_PSGamepad_Look
  (params (ActionValue :type Vector%202D%20Structure) (ElapsedSeconds :type Float%20%28double-precision%29) (TriggeredSeconds :type Float%20%28double-precision%29) (InputAction :type Input%20Action%20Object%20Reference :default "/Game/PlaystationGamepad/IA_PSGamepad_Look.IA_PSGamepad_Look"))
  (:Triggered
    (Class|PlayerController|AddPitchInput (.y ActionValue))
    (Class|PlayerController|AddYawInput (.x ActionValue))))

(event Input|EnhancedActionEvents|EnhancedInputActionIA_PSGamepad_Move
  (params (ActionValue :type Vector :default "0, 0, 0") (ElapsedSeconds :type Float%20%28double-precision%29) (TriggeredSeconds :type Float%20%28double-precision%29) (InputAction :type Input%20Action%20Object%20Reference :default "/Game/PlaystationGamepad/IA_PSGamepad_Move.IA_PSGamepad_Move"))
  (bind _returnvalue (Game|GetPlayerController 0))
  (bind _returnvalue_2 (Pawn|GetControlledPawn _returnvalue))
  (bind _asdefault_pawn (Utilities|Casting|CastToDefaultPawn _returnvalue_2))
  (:Triggered
    (Class|DefaultPawn|MoveRight _asdefault_pawn (.x ActionValue))
    (Class|DefaultPawn|MoveForward _asdefault_pawn (.y ActionValue))
    (Class|DefaultPawn|MoveUpWorld _asdefault_pawn (.z ActionValue))))

(event EventBeginPlay
  (bind _returnvalue (Game|GetPlayerController 0))
  (Class|EnhancedInputSubsystemInterface|AddPlayerMappableConfig (PlayerController|LocalPlayerSubsystems|GetEnhancedInputLocalPlayerSubsystem _returnvalue) "/Game/PlaystationGamepad/IMP_PSGamepad.IMP_PSGamepad" (Utilities|Struct|MakeModifyContextOptions false false))
  (CallFunction|DetectFirstGeneration)
  (CallFunction|LogRegisteredDevices)
  (Input|SetInputModeGameOnly _returnvalue true))

(fn ConstructionScript)

(fn LogRegisteredDevices
  (for (_array_element _array_index) (Class|RawInputFunctionLibrary|GetRegisteredDevices)
    (Development|PrintString (Utilities|String|Append "Handle : " (Utilities|String|ToString(Integer) (.handle _array_element)) "  
" "VendorID : " (Utilities|String|ToString(Integer) (.vendorid _array_element)) "  
" "ProductID : " (Utilities|String|ToString(Integer) (.productid _array_element)) "  
" "DeviceName : " (.devicename _array_element) "  
" "ArrayIndex : " (Utilities|String|ToString(Integer) _array_index)) true true "(R=0.000000,G=0.660000,B=1.000000,A=1.000000)" 5.0)))

(fn DetectFirstGeneration
  (for _array_element (Class|RawInputFunctionLibrary|GetRegisteredDevices)
    (if (Utilities|String|Contains (.devicename _array_element) "05C4")
      (Variables|Default|SetbIsFirstGeneration true)
      (Development|PrintString "!!! FIRST GENERATION DUALSHOCK4 !!!"))))